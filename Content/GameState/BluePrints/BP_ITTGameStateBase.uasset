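; BP_ITTGameStateBase is the game state that reveals the divided-view HUD once role selection completes.
; BeginPlay creates WBP_DividedView and adds it to the viewport hidden.
; When IsRoleSelected replicates as true, its OnRep has BP_May, BP_Cody and BP_EnemyFlyingSaucer create their custom widgets, then shows the divided view.
; An authority-only BP_Rose_Arm spawn is left disconnected and never runs.
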(event EventBeginPlay
  (bind _returnvalue (UserInterface|CreateWidget "/Game/View/Blueprint/WBP_DividedView.WBP_DividedView_C"))
  (bind _output_get (Variables|Default|Setwidget_DividedView _returnvalue))
  (UserInterface|Viewport|AddtoViewport _output_get 0)
  (Widget|SetVisibility _output_get "Hidden"))

(event EventTick
  (params (DeltaSeconds :type Float%20%28single-precision%29)))

(fn ConstructionScript)

(fn OnRepIsRoleSelected
  (if (Variables|Default|GetIsRoleSelected)
    (bind _returnvalue (Actor|GetActorOfClass "/Game/Characters/May/BP/BP_May.BP_May_C"))
    (Default|CreateAllCustomWidgets _returnvalue)
    (bind _returnvalue_2 (Actor|GetActorOfClass "/Game/Characters/Cody/BP/BP_Cody.BP_Cody_C"))
    (Default|CreateAllCustomWidgets _returnvalue_2)
    (bind _returnvalue_3 (Actor|GetActorOfClass "/Game/Characters/EnemyFlyingSaucer/BluePrints/BP_EnemyFlyingSaucer.BP_EnemyFlyingSaucer_C"))
    (Default|CreateAllCustomWidgets _returnvalue_3)
    (Widget|SetVisibility (Variables|Default|Getwidget_DividedView) "Visible")))