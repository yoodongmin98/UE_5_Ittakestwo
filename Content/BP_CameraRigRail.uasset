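; Camera rig rail Blueprint that continuously advances a position along its rail spline in a repeating loop.
; Each Tick adds scaled delta time to CurPos, mirrors it to CurrentPositionOnRail, and wraps CurPos once it passes 1.
; The world location sampled from the spline at that time, without constant velocity, is cached in Pos and exposed through GetPos.
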(event EventBeginPlay)

(event Collision|EventActorBeginOverlap
  (params (OtherActor :type Actor%20Object%20Reference)))

(event EventTick
  (params (DeltaSeconds :type Float%20%28single-precision%29))
  (bind _output_get (Variables|Default|SetCurrentPositionOnRail (+ (* DeltaSeconds 0.1) (Variables|Default|GetCurPos))))
  (bind _output_get_2 (Variables|Default|SetCurPos _output_get))
  (Variables|Default|SetPos (Spline|GetLocationatTime (Class|CameraRigRail|GetRailSplineComponent) _output_get_2 "World" false))
  (if (> _output_get_2 1.0)
    (Variables|Default|SetCurPos (- (Variables|Default|GetCurPos) 1.0))))

(fn ConstructionScript)

(fn GetPos
  (return (Variables|Default|GetPos)))