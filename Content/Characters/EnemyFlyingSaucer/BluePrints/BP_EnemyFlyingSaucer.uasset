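; Flying saucer boss enemy that fires a laser beam and carries interaction prompts for Cody and May.
; BeginPlay spawns a laser FX actor and attaches it and both prompts to mesh sockets; multicast events toggle the beam with sound.
; The beam's aim point lerps between previous and next targets, using blackboard or member values.
; Tick waits for GameState role selection before player setup; other events create boss HP UI and set split-screen with authority.
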(event Custom|ActiveMayInteractionUI
  (params (bNewVisibility :type Boolean) (bPropagateToChildren :type Boolean))
  (Rendering|SetVisibility (Variables|Default|GetMayInteraction) bNewVisibility bPropagateToChildren))

(event Custom|CreateAllCustomWidgets
  (bind _returnvalue (UserInterface|CreateWidget "/Game/UI/Blueprint/WBP_BossHpUIDetail.WBP_BossHpUIDetail_C"))
  (UserInterface|Viewport|AddtoViewport _returnvalue 0))

(event Custom|ActiveCodyInteractionUI
  (params (bNewVisibility :type Boolean) (bPropagateToChildren :type Boolean))
  (bind _codyinteraction (Variables|Default|GetCodyInteraction))
  (bind _codyinteraction_2 (Variables|Default|GetCodyInteraction))
  (bind _widgetinstance (Variables|/Script/UE5_ITT.InteractionWidget|GetWidgetInstance _codyinteraction))
  (Utilities|IsValid _widgetinstance
    (:Is%20Valid
      (if bNewVisibility
        (Widget|SetVisibility _widgetinstance "Visible")
        (Variables|/Script/UE5_ITT.InteractionWidget|SetbIsViewWiget _codyinteraction_2 true)
        (else
          (Widget|SetVisibility _widgetinstance "Hidden")
          (Variables|/Script/UE5_ITT.InteractionWidget|SetbIsViewWiget _codyinteraction_2 false))))))

(event Custom|MultiCast_ChaseLaserBeam
  (bind _laserfxspawn (Variables|Default|GetLaserFXSpawn))
  (Utilities|IsValid _laserfxspawn
    (:Is%20Valid
      (Variables|/Game/Map/FX/Laser/BP_LaserFXParent.BP_LaserFXParent_C|SetAttackActorPos _laserfxspawn (Math|Vector|Lerp(Vector) (Variables|Default|GetPrevLaserTargetLocation) (Variables|Default|GetNextLaserTargetLocation) (Variables|Default|GetLaserLerpRatio))))))

(event Custom|MultiCast_InActiveLaserFXSpawn
  (CallFunction|InActiveLaserFXSpawn))

(event Custom|ActiveSplitScreenMode
  (params (bActive :type Boolean))
  (bind _asbp_ittgame_state_base (Utilities|Casting|CastToBP_ITTGameStateBase (Game|GetGameState)))
  (if (Ability|HasAuthority _asbp_ittgame_state_base)
    (Default|SplitscreenMode _asbp_ittgame_state_base bActive)))

(event Custom|MultiCast_ActiveLaserFXSpawn
  (CallFunction|ActiveLaserFXSpawn))

(event EventBeginPlay
  (CallFunction|CreateLaserFXSpawn))

(event Collision|EventActorBeginOverlap
  (params (OtherActor :type Actor%20Object%20Reference)))

(event EventTick
  (params (DeltaSeconds :type Float%20%28single-precision%29))
  (if (Variables|Default|GetbIsFsmStart)
    ;[1 1 1] 컷신 Start 체크 후 위젯 ON,OFF 처리
    (if (Variables|Default|GetbIsCutSceneStart)
      _)
    (else
      (bind _asbp_ittgame_state_base (Utilities|Casting|CastToBP_ITTGameStateBase (Game|GetGameState)))
      (if (Variables|/Game/GameState/BluePrints/BP_ITTGameStateBase.BP_ITTGameStateBase_C|GetIsRoleSelected _asbp_ittgame_state_base)
        (Variables|Default|SetbIsFsmStart true)
        (Class|EnemyFlyingSaucer|SetupPlayerActorsCodyandMay self)))))

(fn ConstructionScript)

(fn ChaseLaserBeam
  (bind _returnvalue (Pawn|GetController))
  (bind _laserfxspawn (Variables|Default|GetLaserFXSpawn))
  (bind _returnvalue_2 (AI|GetBlackboard _returnvalue))
  (Utilities|IsValid _laserfxspawn
    (:Is%20Valid
      (Variables|/Game/Map/FX/Laser/BP_LaserFXParent.BP_LaserFXParent_C|SetAttackActorPos _laserfxspawn (Math|Vector|Lerp(Vector) (AI|Components|Blackboard|GetValueasVector _returnvalue_2 (Variables|Default|GetPrev%20Laser%20Attack%20Location%20Name)) (AI|Components|Blackboard|GetValueasVector _returnvalue_2 (Variables|Default|GetPrevTargetLocation%20Name)) (Class|BlackboardComponent|GetValueasFloat _returnvalue_2 (Variables|Default|GetLaserLerpRatio%20Name)))))))

(fn ActiveLaserFXSpawn
  (bind _laserfxspawn (Variables|Default|GetLaserFXSpawn))
  (Utilities|IsValid _laserfxspawn
    (:Is%20Valid
      (Variables|/Game/Map/FX/Laser/BP_LaserFXParent.BP_LaserFXParent_C|SetbActiveLaser _laserfxspawn true)
      (Audio|PlaySound2D "/Game/Sound/Boss/Cue/Laser/SC_LaserStart.SC_LaserStart" 1.0 1.0 0.0 0 0))
    (:Is%20Not%20Valid
      (Development|PrintString "LaserFXSpawn is Not Valid"))))

(fn InActiveLaserFXSpawn
  (bind _laserfxspawn (Variables|Default|GetLaserFXSpawn))
  (Utilities|IsValid _laserfxspawn
    (:Is%20Valid
      (Variables|/Game/Map/FX/Laser/BP_LaserFXParent.BP_LaserFXParent_C|SetbActiveLaser _laserfxspawn false)
      (Audio|PlaySound2D "/Game/Sound/Boss/Cue/Laser/SC_LaserEnd.SC_LaserEnd" 1.0 1.0 0.0 0 0))))

(fn CreateLaserFXSpawn
  (bind _self self)
  (bind _self_2 self)
  (bind _mesh (Variables|Character|GetMesh _self))
  (Variables|Default|SetFlyingSaucerAIController (Pawn|GetController))
  (bind _returnvalue (Game|SpawnActorfromClass "/Game/Map/FX/Laser/BP_LaserFXSpawn.BP_LaserFXSpawn_C" (Math|Transform|MakeTransform "0, 0, 0" (Transformation|GetActorRotation _self_2) "1.000000,1.000000,1.000000") "Undefined" "MultiplyWithRoot" _self_2 "(R=0.984375,G=0.066650,B=0.066650,A=1.000000)" 0 "0.000000,0.000000,0.000000" true 0))
  (Variables|Default|SetLaserFXSpawn _returnvalue)
  (Variables|/Game/Map/FX/Laser/BP_LaserFXParent.BP_LaserFXParent_C|SetbActiveLaser _returnvalue (Variables|Default|GetbDefaultLaserState))
  (Transformation|AttachComponentToComponent _returnvalue _mesh "LaserSpawnPointSocket" "KeepRelative" "KeepRelative" "KeepRelative" true)
  (Transformation|AttachComponentToComponent (Variables|Default|GetMayInteraction) _mesh "MayUISocket" "KeepRelative" "KeepRelative" "KeepRelative" true)
  (Transformation|AttachComponentToComponent (Variables|Default|GetCodyInteraction) _mesh "CodyUISocket" "KeepRelative" "KeepRelative" "KeepRelative" true)
  (CallFunction|ActiveMayInteractionUI false true))

(fn SettingView
  (if (Actor|ActorHasTag (Game|Player|GetPlayerPawn 0) "Cody")
    _))