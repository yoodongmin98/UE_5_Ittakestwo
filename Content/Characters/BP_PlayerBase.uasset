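; Placeholder player for two-player networked role selection, letting host and client choose between Cody and May through WBP_RoleSelectionUI.
; Left/Right set each user's next slot, branching on authority, with client input routed through events.
; RepNotify on those slots animates the widget and commits the selection.
; Enter possesses the chosen character's existing actor and, once both users finish, destroys all BP_PlayerBase actors; a numpad key toggles the UI.
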(event Custom|ClientPressLeft
  ;[1 1 1] Character Selection
  (CallFunction|ReplicateEventUser2))

(event Custom|ClientPressRIght
  ;[1 1 1] Character Selection
  (CallFunction|ReplicateEventUser1))

(event Custom|ChangeUser2
  (params (role :type Integer))
  (bind _returnvalue (Game|GetPlayerController 1))
  (switch int role
    (:1
      (bind _returnvalue_2 (Actor|GetActorOfClass "/Game/Characters/Cody/BP/BP_Cody.BP_Cody_C"))
      (Pawn|Possess _returnvalue _returnvalue_2)
      (Variables|Default|SetChangeDone2 true)
      (CallFunction|DestroyBaseBPPlayer))
    (:2
      (bind _returnvalue_3 (Actor|GetActorOfClass "/Game/Characters/May/BP_May.BP_May_C"))
      (Pawn|Possess _returnvalue _returnvalue_3)
      (Variables|Default|SetChangeDone2 true)
      (CallFunction|DestroyBaseBPPlayer))))

(event Custom|DestroyBaseBP_Player
  (if (Variables|Default|GetChangeDone%201)
    (if (Variables|Default|GetChangeDone2)
      (bind _outactors (Actor|GetAllActorsOfClass "BP_PlayerBase_C"))
      (Actor|DestroyActor _outactors))))

(event EventBeginPlay
  (bind _foundwidgets (Widget|GetAllWidgetsOfClass "/Game/UI/WBP_RoleSelectionUI.WBP_RoleSelectionUI_C" true))
  (Utilities|IsValid (Utilities|Array|Get(acopy) _foundwidgets)
    (:Is%20Valid
      (bind _output_get (Variables|Default|SetWidget%20UI (Utilities|Array|Get(acopy) _foundwidgets)))
      (Widget|SetVisibility _output_get "Visible")
      (Variables|Default|SetView%20Widget%20UI true))))

(event Collision|EventActorBeginOverlap
  (params (OtherActor :type Actor%20Object%20Reference)))

(event EventTick
  (params (DeltaSeconds :type Float%20%28single-precision%29)))

(event Input|KeyboardEvents|Left
  (params (Key :type Key%20Structure :default "None"))
  ;[1 1 1] Character Selection
  (:Pressed
    (Utilities|IsValid (Variables|Default|GetWidget%20UI)
      (:Is%20Valid
        (CallFunction|SelectLeft)))))

(event Input|KeyboardEvents|Right
  (params (Key :type Key%20Structure :default "None"))
  ;[1 1 1] Character Selection
  (:Pressed
    (Utilities|IsValid (Variables|Default|GetWidget%20UI)
      (:Is%20Valid
        (CallFunction|SelectRight)))))

(event Input|KeyboardEvents|NumPadNine
  (params (Key :type Key%20Structure :default "None"))
  ;[1 1 1] Character Selection
  (:Pressed
    (Utilities|IsValid (Variables|Default|GetWidget%20UI)
      (:Is%20Valid
        (CallFunction|SetVisibilityUIFuc)))))

(event Input|KeyboardEvents|Enter
  (params (Key :type Key%20Structure :default "None"))
  (:Pressed
    (Networking|SwitchHasAuthority
      (:Authority
        (CallFunction|ChangeUser1))
      (:Remote
        (CallFunction|ChangeUser2 (Variables|Default|GetCurUser2))))))

(fn ConstructionScript)

(fn SelectLeft
  (Networking|SwitchHasAuthority
    (:Authority
      (switch int (Variables|Default|GetCur%20User%201)
        (:0
          (Variables|Default|SetNextUser1 2))
        (:1
          (Variables|Default|SetNextUser1 0))))
    (:Remote
      (CallFunction|ClientPressLeft))))

(fn SelectRight
  (Networking|SwitchHasAuthority
    (:Authority
      (switch int (Variables|Default|GetCur%20User%201)
        (:0
          (Variables|Default|SetNextUser1 1))
        (:2
          (Variables|Default|SetNextUser1 0))))
    (:Remote
      (CallFunction|ClientPressRIght))))

(fn ReplicateEventUser2
  (switch int (Variables|Default|GetCurUser2)
    (:0
      (Variables|Default|SetNextUser2 2))
    (:1
      (Variables|Default|SetNextUser2 0))))

(fn ReplicateEventUser1
  (switch int (Variables|Default|GetCurUser2)
    (:0
      (Variables|Default|SetNextUser2 1))
    (:2
      (Variables|Default|SetNextUser2 0))))

(fn SetVisibilityUIFuc
  (if (Variables|Default|GetView%20Widget%20UI)
    (Widget|SetVisibility (Variables|Default|GetWidget%20UI) "Hidden")
    (Variables|Default|SetView%20Widget%20UI false)
    (else
      (Widget|SetVisibility (Variables|Default|GetWidget%20UI) "Visible")
      (Variables|Default|SetView%20Widget%20UI true))))

(fn OnRepNextUser1
  (bind _widget_ui (Variables|Default|GetWidget%20UI))
  (bind _widget_ui_2 (Variables|Default|GetWidget%20UI))
  (Networking|SwitchHasAuthority
    (:Authority
      (Utilities|IsValid _widget_ui
        (:Is%20Valid
          (Default|MainUIAnimation _widget_ui (Variables|Default|GetCur%20User%201) (Variables|Default|GetNextUser1) true)
          (Variables|Default|SetCur%20User%201 (Variables|Default|GetNextUser1)))))
    (:Remote
      (if (Utilities|IsValid _widget_ui_2)
        (Default|MainUIAnimation _widget_ui_2 (Variables|Default|GetCur%20User%201) (Variables|Default|GetNextUser1) true)
        (Variables|Default|SetCur%20User%201 (Variables|Default|GetNextUser1))))))

(fn OnRepNextUser2
  (bind _widget_ui (Variables|Default|GetWidget%20UI))
  (Networking|SwitchHasAuthority
    (:Authority
      (Default|MainUIAnimation (Variables|Default|GetWidget%20UI) (Variables|Default|GetCurUser2) (Variables|Default|GetNextUser2) false)
      (Variables|Default|SetCurUser2 (Variables|Default|GetNextUser2)))
    (:Remote
      (Utilities|IsValid _widget_ui
        (:Is%20Valid
          (Default|MainUIAnimation _widget_ui (Variables|Default|GetCurUser2) (Variables|Default|GetNextUser2) false)
          (Variables|Default|SetCurUser2 (Variables|Default|GetNextUser2)))))))

(fn ChangeUser1
  (bind _returnvalue (Game|GetPlayerController 0))
  (switch int (Variables|Default|GetCur%20User%201)
    (:1
      (Actor|GetActorOfClass "/Game/Characters/Cody/BP/BP_Cody.BP_Cody_C")
      (Pawn|Possess _returnvalue)
      (Variables|Default|SetChangeDone%201 true)
      (CallFunction|DestroyBaseBPPlayer))
    (:2
      (bind _returnvalue_2 (Actor|GetActorOfClass "/Game/Characters/May/BP_May.BP_May_C"))
      (Pawn|Possess _returnvalue _returnvalue_2)
      (Variables|Default|SetChangeDone%201 true)
      (CallFunction|DestroyBaseBPPlayer))))