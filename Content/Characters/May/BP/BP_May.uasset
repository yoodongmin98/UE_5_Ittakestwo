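; BP_May is the Blueprint for the playable character May, handling input setup, health UI, death and homing exit.
; BeginPlay adds the IMC_Cody mapping context, while custom events create the HP widget and assign the scene capture render target.
; Tick feeds the HP ratio into the widget material, swaps the mesh for a one-time Niagara death effect, and launches May backward off homing overlaps.
; F9 triggers a test attack.
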(event Custom|SetTarget
  (Variables|/Script/Engine.SceneCaptureComponent2D|SetTextureTarget (Variables|Default|GetSceneCaptureComponent2D) "/Game/View/Material/MayRenderTarget.MayRenderTarget"))

(event Custom|CreateAllCustomWidgets
  (bind _returnvalue (UserInterface|CreateWidget "/Game/UI/Blueprint/WBP_MayHpUI.WBP_MayHpUI_C"))
  (UserInterface|Viewport|AddtoViewport _returnvalue 0)
  (Variables|Default|SetPlayerHpWidget _returnvalue))

(event EventBeginPlay
  ;[1 1 1] Begin Play
  (CallFunction|ImportController))

(event EventTick
  (params (DeltaSeconds :type Float%20%28single-precision%29))
  ;[1 1 1] Event Tick
  (CallFunction|HPWidgetFunction)
  (CallFunction|DeathParticle)
  (CallFunction|GetOffHoming))

(event Input|KeyboardEvents|F9
  (params (Key :type Key%20Structure :default "None"))
  ;[1 1 1] Test Attack
  (:Pressed
    (Class|PlayerBase|AttackPlayer 1)
    (Default|AttackEvent (Variables|Default|GetPlayerHpWidget))))

(fn ConstructionScript)

(fn HPWidgetFunction
  (bind _playerhpwidget (Variables|Default|GetPlayerHpWidget))
  (Utilities|IsValid _playerhpwidget
    (:Is%20Valid
      (bind _returnvalue (Appearance|GetDynamicMaterial (Variables|/Game/UI/Blueprint/WBP_MayHpUI.WBP_MayHpUI_C|GetwbPlayerHpImage _playerhpwidget) :!class /Script/UMG.Image))
      (Rendering|Material|SetScalarParameterValue _returnvalue "bHpParameter" (/ (Math|Conversions|ToFloat(Integer) (Class|PlayerBase|GetPlayerHP)) (Class|PlayerBase|GetPlayerFullHP)) :!class /Script/Engine.MaterialInstanceDynamic))))

(fn DeathParticle
  (if (Class|PlayerBase|GetIsPlayerDeath)
    (if (not (Variables|Default|GetDeath%20Bool))
      (AddComponent|AddNiagaraComponent false (Math|Transform|MakeTransform (+ (Math|Vector|GetUpVector (Variables|Character|GetMesh)) "0.000000,0.000000,150.000000") "0, 0, 0" "1.000000,1.000000,1.000000"))
      (Variables|Default|SetDeath%20Bool true)
      (Rendering|SetVisibility (Variables|Character|GetMesh) false false)
      (Class|PlayerBase|SetCodyHoldEnemyTrue))))

(fn ImportController
  (bind _as플레이어_컨트롤러 (Utilities|Casting|CastToPlayerController (Pawn|GetController)))
  (Input|AddMappingContext (PlayerController|LocalPlayerSubsystems|GetEnhancedInputLocalPlayerSubsystem _as플레이어_컨트롤러) "/Game/Characters/Cody/BP/Input/IMC_Cody.IMC_Cody" 0 "(bIgnoreAllPressedKeysUntilRelease=True,bForceImmediately=False,bNotifyUserSettings=False)"))

(fn GetOffHoming
  (if (Class|PlayerBase|GetOverlapHoming)
    (Class|PlayerBase|SetFlyFalse)
    (Character|LaunchCharacter (+ (* (* (Transformation|GetActorForwardVector) "-1.000000,-1.000000,-1.000000") 5e+02) (Math|Vector|MakeVector 0.0 0.0 (Variables|/Script/Engine.CharacterMovementComponent|GetJumpZVelocity (Variables|Character|GetCharacterMovement)))) true true)
    (Class|PlayerBase|SetOverlapHoming)
    (Class|PlayerBase|SpringArmDefaultFunction)))