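; Player character Blueprint for Cody, handling movement, health UI and death/respawn.
; Tick runs a forward-trace wall slide that feeds wall jumps, plus a launch off homing overlaps.
; Tick also copies inherited HP and death state into RepNotify variables, whose handlers update material gauges and swap HP and respawn widgets.
; Death spawns Niagara and hides the mesh until full HP restores it at the respawn position.
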(event Custom|SetTarget
  ;[1 1 1] RenderTargetSetting
  (Variables|/Script/Engine.SceneCaptureComponent2D|SetTextureTarget (Variables|Default|GetSceneCaptureComponent2D) "/Game/View/Material/CodyRenderTarget.CodyRenderTarget"))

(event Custom|CreateAllCustomWidgets
  ;[1 1 1] Widget 생성
  (bind _returnvalue (UserInterface|CreateWidget "/Game/UI/Blueprint/WBP_CodyHpUI.WBP_CodyHpUI_C"))
  (UserInterface|Viewport|AddtoViewport _returnvalue 0)
  (Variables|Default|SetPlayerHpWidget _returnvalue)
  (bind _returnvalue_2 (UserInterface|CreateWidget "/Game/UI/Blueprint/WBP_Respawn.WBP_Respawn_C"))
  (UserInterface|Viewport|AddtoViewport _returnvalue_2 0)
  (bind _output_get (Variables|Default|SetRespawnUI _returnvalue_2))
  (Class|UserWidget|SetPositioninViewport _output_get "(X=320.000000,Y=0.000000)" true)
  (Widget|SetVisibility _output_get "Hidden"))

(event Custom|SetServerUIVisible
  ;[1 1 1] UIVisibleSetting
  (CallFunction|SetMultiUIVisible))

(event Custom|SetMultiUIVisible
  (bind _playerhpwidget (Variables|Default|GetPlayerHpWidget))
  (bind _respawnui (Variables|Default|GetRespawnUI))
  (bind _playerhpwidget_2 (Variables|Default|GetPlayerHpWidget))
  (bind _respawnui_2 (Variables|Default|GetRespawnUI))
  ;[1 1 1] UIVisibleSetting
  (if (Class|PlayerBase|GetIsPlayerDeath)
    (Utilities|IsValid _playerhpwidget
      (:Is%20Valid
        (Widget|SetVisibility _playerhpwidget "Hidden")
        (Utilities|IsValid _respawnui
          (:Is%20Valid
            (Widget|SetVisibility _respawnui "Visible")))))
    (else
      (Utilities|IsValid _playerhpwidget_2
        (:Is%20Valid
          (Widget|SetVisibility _playerhpwidget_2 "Visible")
          (Utilities|IsValid _respawnui_2
            (:Is%20Valid
              (Widget|SetVisibility _respawnui_2 "Hidden"))))))))

(event Input|EnhancedActionEvents|EnhancedInputActionIA_Jump
  (params (ActionValue :type Boolean) (ElapsedSeconds :type Float%20%28double-precision%29) (TriggeredSeconds :type Float%20%28double-precision%29) (InputAction :type Input%20Action%20Object%20Reference :default "/Game/Characters/Cody/BP/Input/IA_Jump.IA_Jump"))
  ;[1 1 1] Jump Event
  (:Started
    (if (Variables|Default|GetbIsWallSlide)
      (CallFunction|WallJumpFunction)
      (else
        (Character|Jump))))
  (:Completed
    (Character|StopJumping)))

(event EventBeginPlay
  ;[1 1 1] BeginPlay
  (CallFunction|ImpotController,Widget))

(event EventTick
  (params (DeltaSeconds :type Float%20%28single-precision%29))
  ;[1 1 1] Event Tick
  (CallFunction|WallSlideFunction)
  (CallFunction|PlayerHpFunction)
  (CallFunction|GetOffHoming)
  (CallFunction|DeathParticle))

(event Input|KeyboardEvents|F9
  (params (Key :type Key%20Structure :default "None"))
  ;[1 1 1] Test Attack
  (:Pressed
    (Class|PlayerBase|AttackPlayer 1)))

(event Input|KeyboardEvents|E
  (params (Key :type Key%20Structure :default "None")))

(fn ConstructionScript)

(fn WallSlideFunction
  (bind _returnvalue (Transformation|GetActorLocation))
  (bind _charactermovement (Variables|Character|GetCharacterMovement))
  (if (AI|Components|NavMovement|IsFalling (Variables|Character|GetCharacterMovement))
    (bind (_outhit _returnvalue_2) (Collision|LineTraceByChannel _returnvalue (+ _returnvalue (* (Transformation|GetActorForwardVector) 5.0)) "TraceTypeQuery1" false 0 "None"))
    (if _returnvalue_2
      (Variables|Default|SetbIsWallSlide true)
      (Transformation|SetActorRotation (Math|Rotator|MakeRotator 0.0 0.0 (+ (.yaw (Math|Conversions|RotationFromXVector (.ImpactNormal (Collision|BreakHitResult _outhit)))) 1.8e+02)))
      (Variables|/Script/Engine.MovementComponent|SetVelocity _charactermovement (Math|Interpolation|VInterptoConstant (Variables|/Script/Engine.MovementComponent|GetVelocity _charactermovement) "0, 0, 0" (Utilities|Time|GetWorldDeltaSeconds) 2e+03))
      (else
        (Variables|Default|SetbIsWallSlide false)))))

(fn ImpotController,Widget
  (bind _as플레이어_컨트롤러 (Utilities|Casting|CastToPlayerController (Pawn|GetController)))
  (Input|AddMappingContext (PlayerController|LocalPlayerSubsystems|GetEnhancedInputLocalPlayerSubsystem _as플레이어_컨트롤러) "/Game/Characters/Cody/BP/Input/IMC_Cody.IMC_Cody" 0 "(bIgnoreAllPressedKeysUntilRelease=True,bForceImmediately=False,bNotifyUserSettings=False)")
  (Variables|Default|SetPlayerHpUI (Class|PlayerBase|GetPlayerHP))
  (Variables|Default|SetIsDeathNotify (Class|PlayerBase|GetIsPlayerDeath)))

(fn PlayerHpFunction
  (if (== (Class|PlayerBase|GetPlayerHP) (Variables|Default|GetPlayerHpUI))
    _
    (else
      (Variables|Default|SetPlayerHpUI (Class|PlayerBase|GetPlayerHP))))
  (if (not (== (Class|PlayerBase|GetIsPlayerDeath) (Variables|Default|GetIsDeathNotify)))
    (Variables|Default|SetIsDeathNotify (Class|PlayerBase|GetIsPlayerDeath))))

(fn WallJumpFunction
  (Transformation|SetActorRotation (Math|Rotator|MakeRotator 0.0 0.0 (+ (.yaw (Transformation|GetActorRotation)) 1.8e+02)))
  (Character|LaunchCharacter (+ (* (Transformation|GetActorForwardVector) 1.5e+02) (Math|Vector|MakeVector 0.0 0.0 (Variables|/Script/Engine.CharacterMovementComponent|GetJumpZVelocity (Variables|Character|GetCharacterMovement)))) true true))

(fn GetOffHoming
  (if (Class|PlayerBase|GetOverlapHoming)
    (Class|PlayerBase|SetFlyFalse)
    (Character|LaunchCharacter (+ (* (* (Transformation|GetActorForwardVector) "-1.000000,-1.000000,-1.000000") 5e+02) (Math|Vector|MakeVector 0.0 0.0 (Variables|/Script/Engine.CharacterMovementComponent|GetJumpZVelocity (Variables|Character|GetCharacterMovement)))) true true)
    (Class|PlayerBase|SetOverlapHoming)
    (Class|PlayerBase|SpringArmDefaultFunction)))

(fn CutSceneAnimation
  (if (Class|Cody|GetCutScenceTrigger)
    (Components|Animation|PlayAnimation (Variables|Character|GetMesh) "/Game/Characters/Cody/Animation/Behaviour/PlayRoom/CutScene/PlayRoom_SpaceStation_BossFight_LaserRippedOff_Cody_Anim1.PlayRoom_SpaceStation_BossFight_LaserRippedOff_Cody_Anim1" false)))

(fn DeathParticle
  (if (Class|PlayerBase|GetIsPlayerDeath)
    (if (Variables|Default|GetDeath%20Bool)
      (if (not (Rendering|IsVisible (Variables|Character|GetMesh)))
        (if (== (Class|PlayerBase|GetPlayerHP) (Class|PlayerBase|GetPlayerFullHP))
          (if (not (Variables|Default|GetResPawnBool))
            (Variables|Default|SetResPawnBool true)
            (Class|Cody|SetCodyMoveable)
            (Rendering|SetVisibility (Variables|Character|GetMesh) true false)
            (Collision|SetActorEnableCollision true) ; 되는건지 안되는건지 모름 ㄹㅇ
            (Variables|Default|SetDeath%20Bool false)
            (bind _returnvalue (Class|PlayerBase|GetResPawnPosition))
            (Transformation|SetActorLocation _returnvalue false false))))
      (else
        (AddComponent|AddNiagaraComponent false (Math|Transform|MakeTransform (+ (Math|Vector|GetUpVector (Variables|Character|GetMesh)) "0.000000,0.000000,150.000000") "0, 0, 0" "1.000000,1.000000,1.000000"))
        (Variables|Default|SetDeath%20Bool true)
        (Rendering|SetVisibility (Variables|Character|GetMesh) false false)
        (Class|PlayerBase|SetCodyHoldEnemyTrue)
        (Collision|SetActorEnableCollision false) ; 되는건지 안되는건지 모름 ㄹㅇ
        (Variables|Default|SetResPawnBool false)))))

(fn OnRepPlayerHpUI
  (if (Class|PlayerBase|GetIsPlayerDeath)
    (CallFunction|RespawnUIAnimation)
    (else
      (CallFunction|HPUIAnimation))))

(fn HPUIAnimation
  (bind _playerhpwidget (Variables|Default|GetPlayerHpWidget))
  (Utilities|IsValid _playerhpwidget
    (:Is%20Valid
      (bind _returnvalue (Appearance|GetDynamicMaterial (Variables|/Game/UI/Blueprint/WBP_CodyHpUI.WBP_CodyHpUI_C|GetwbPlayerHpImage _playerhpwidget) :!class /Script/UMG.Image))
      (Rendering|Material|SetScalarParameterValue _returnvalue "bHpParameter" (/ (Math|Conversions|ToFloat(Integer) (Class|PlayerBase|GetPlayerHP)) (Class|PlayerBase|GetPlayerFullHP)) :!class /Script/Engine.MaterialInstanceDynamic)
      (Default|AttackEvent (Variables|Default|GetPlayerHpWidget)))))

(fn RespawnUIAnimation
  (bind _respawnui (Variables|Default|GetRespawnUI))
  (Utilities|IsValid _respawnui
    (:Is%20Valid
      (bind _returnvalue (Appearance|GetDynamicMaterial (Variables|/Game/UI/Blueprint/WBP_Respawn.WBP_Respawn_C|GetwbRespawnGage _respawnui) :!class /Script/UMG.Image))
      (Rendering|Material|SetScalarParameterValue _returnvalue "RespawnParamter" (/ (Math|Conversions|ToFloat(Integer) (Class|PlayerBase|GetPlayerHP)) (Class|PlayerBase|GetPlayerFullHP)) :!class /Script/Engine.MaterialInstanceDynamic)
      (Default|PressRespawn _respawnui))))

(fn OnRepIsDeathNotify
  (bind _playerhpwidget (Variables|Default|GetPlayerHpWidget))
  (bind _respawnui (Variables|Default|GetRespawnUI))
  (bind _playerhpwidget_2 (Variables|Default|GetPlayerHpWidget))
  (bind _respawnui_2 (Variables|Default|GetRespawnUI))
  (if (Variables|Default|GetIsDeathNotify)
    (Utilities|IsValid _playerhpwidget
      (:Is%20Valid
        (Widget|SetVisibility _playerhpwidget "Hidden")
        (Utilities|IsValid _respawnui
          (:Is%20Valid
            (Widget|SetVisibility _respawnui "Visible")
            (CallFunction|RespawnUIAnimation)))))
    (else
      (Utilities|IsValid _playerhpwidget_2
        (:Is%20Valid
          (Widget|SetVisibility _playerhpwidget_2 "Visible")
          (Utilities|IsValid _respawnui_2
            (:Is%20Valid
              (Widget|SetVisibility _respawnui_2 "Hidden")
              (CallFunction|HPUIAnimation))))))))