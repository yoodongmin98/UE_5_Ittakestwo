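; BP_Cody is the Cody character Blueprint, which passes Left and Right key presses to a shared UI replication actor.
; On BeginPlay it adds the IMC_Cody Enhanced Input mapping context and caches the BP_UIReplicateActor found in the level.
; Raw key events switch on authority, calling that actor's PressServer functions on the authority side and its Press event variants on remotes.
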(event EventBeginPlay
  (bind _as플레이어_컨트롤러 (Utilities|Casting|CastToPlayerController (Pawn|GetController)))
  (Input|AddMappingContext (PlayerController|LocalPlayerSubsystems|GetEnhancedInputLocalPlayerSubsystem _as플레이어_컨트롤러) "/Game/Characters/Cody/Control/Input/IMC_Cody.IMC_Cody" 0 "(bIgnoreAllPressedKeysUntilRelease=True,bForceImmediately=False,bNotifyUserSettings=False)")
  (bind _returnvalue (Actor|GetActorOfClass "/Game/UI/BP_UIReplicateActor.BP_UIReplicateActor_C"))
  (Variables|Default|SetUIController _returnvalue))

(event Collision|EventActorBeginOverlap
  (params (OtherActor :type Actor%20Object%20Reference)))

(event EventTick
  (params (DeltaSeconds :type Float%20%28single-precision%29)))

(event Input|KeyboardEvents|Left
  (params (Key :type Key%20Structure :default "None"))
  (bind _uicontroller (Variables|Default|GetUIController))
  (:Pressed
    (Networking|SwitchHasAuthority
      (:Authority
        (Default|PressServerLeft _uicontroller))
      (:Remote
        (Default|PressLeftEvent _uicontroller)))))

(event Input|KeyboardEvents|Right
  (params (Key :type Key%20Structure :default "None"))
  (bind _uicontroller (Variables|Default|GetUIController))
  (:Pressed
    (Networking|SwitchHasAuthority
      (:Authority
        (Default|PressServerRight _uicontroller))
      (:Remote
        (Default|PressRightEvent _uicontroller)))))

(fn ConstructionScript)