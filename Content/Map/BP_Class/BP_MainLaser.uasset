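; BP_MainLaser is a laser emitter actor that triggers the explosion of any BP_EnergyCore its beams hit.
; On BeginPlay it spawns a red BP_LaserFXSpawn at every LaserMesh socket, attaches it and leaves it inactive.
; Tick polls each spawner's hit actor and calls SetExplode on energy cores.
; SetActiveLaser and SetLaserSize events pass the active state and size to all spawned lasers.
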(event EventBeginPlay
  (bind _output_get (Variables|Default|SetArray (Transformation|GetAllSocketNames (Variables|Default|GetLaserMesh))))
  (for _array_element _output_get
    (bind _returnvalue (Game|SpawnActorfromClass "/Game/Map/FX/Laser/BP_LaserFXSpawn.BP_LaserFXSpawn_C" (Math|Transform|MakeTransform "0, 0, 0" "0, 0, 0" "1.000000,1.000000,1.000000") "Undefined" "MultiplyWithRoot" 0 "(R=1.000000,G=0.000000,B=0.000000,A=1.000000)" 0 "0.000000,0.000000,0.000000" false 0))
    (Utilities|Array|Add (Variables|Default|GetLaserSpawner) _returnvalue)
    (Transformation|AttachComponentToComponent _returnvalue (Variables|Default|GetLaserMesh) _array_element "KeepRelative" "KeepRelative" "KeepRelative" false)
    (Variables|/Game/Map/FX/Laser/BP_LaserFXParent.BP_LaserFXParent_C|SetbActiveLaser _returnvalue false)))

(event Collision|EventActorBeginOverlap
  (params (OtherActor :type Actor%20Object%20Reference)))

(event EventTick
  (params (DeltaSeconds :type Float%20%28single-precision%29))
  (for _array_element (Variables|Default|GetLaserSpawner)
    (bind _hitactor (Default|GetHitActor _array_element))
    (bind _asbp_energy_core (Utilities|Casting|CastToBP_EnergyCore _hitactor))
    (Utilities|String|LogString (Utilities|GetDisplayName _hitactor))
    (Class|EnergyCore|SetExplode _asbp_energy_core)))

(event EventSetLaserSize
  (params (SizeParam :type Float%20%28single-precision%29))
  (for _array_element (Variables|Default|GetLaserSpawner)
    (Default|SetChildLaserSize _array_element SizeParam)))

(event EventSetActiveLaser
  (params (bValue :type Boolean))
  (for _array_element (Variables|Default|GetLaserSpawner)
    (Variables|/Game/Map/FX/Laser/BP_LaserFXParent.BP_LaserFXParent_C|SetbActiveLaser _array_element bValue)))

(fn ConstructionScript)