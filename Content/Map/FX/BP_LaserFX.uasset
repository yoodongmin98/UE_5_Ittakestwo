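; BP_LaserFX is a laser beam effect actor tinted by a dynamic material instance created at BeginPlay.
; Each tick it snaps to an Arrow's location, pointing its Z axis at the attack target or copying its spawn reference's rotation.
; A thin box trace along the end vector, refreshed from actor forward only without a target, stretches the mesh's Z scale to the hit distance or full range.
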(event EventBeginPlay
  (CallFunction|ChangeColor))

(event EventTick
  (params (DeltaSeconds :type Float%20%28single-precision%29))
  (if (Variables|Default|GetbAttackActor)
    (Variables|Default|SetMyRotation (Math|Rotator|MakeRotfromZ (- (Variables|Default|GetAttackActorPos) (Transformation|GetActorLocation))))
    (else
      (Variables|Default|SetEndvector (Transformation|GetActorForwardVector))
      (Variables|Default|SetMyRotation (Transformation|GetWorldRotation (Variables|/Script/Engine.Actor|GetRootComponent (Variables|Default|GetSpawnReference))))))
  (Transformation|SetActorTransform (Math|Transform|MakeTransform (Transformation|GetWorldLocation (Variables|Default|GetArrow)) (Variables|Default|GetMyRotation) "1.000000,1.000000,1.000000"))
  (CallFunction|SetEndPoint))

(fn ConstructionScript
  (|CallParentFunction))

(fn ChangeColor
  (bind _returnvalue (Rendering|Material|CreateDynamicMaterialInstance (Variables|Default|GetSM_Parent) 0 "/Game/Map/FX/M_LaserFX.M_LaserFX" "None" :!class /Script/Engine.PrimitiveComponent))
  (Rendering|Material|SetVectorParameterValue _returnvalue "Color" (Variables|Default|GetLaserColor) :!class /Script/Engine.MaterialInstanceDynamic))

(fn SetEndPoint
  (bind _returnvalue (Transformation|GetActorLocation))
  (bind _outhit (Collision|BoxTraceByChannel _returnvalue (+ _returnvalue (* (Variables|Default|GetEndvector) (LocalVariables|GetLaserRange))) "0.500000,0.500000,0.500000" "0, 0, 0" "TraceTypeQuery1" false 0 "None"))
  (bind _output_get (LocalVariables|SetLaserHitInfo _outhit))
  (LocalVariables|SetLocalHitActor (.HitActor (Collision|BreakHitResult _output_get)))
  (Transformation|SetWorldScale3D (Variables|Default|GetSM_Parent) (Math|Vector|MakeVector 0.3 0.3 (Math|Float|SelectFloat (/ (+ (.Distance (Collision|BreakHitResult _output_get)) 1.0) 1e+02) (/ (LocalVariables|GetLaserRange) 1e+02) (.bBlockingHit (Collision|BreakHitResult _output_get))))))