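; BP_LaserFXSpawn is a laser spawner actor that owns one BP_LaserFX instance and switches it on and off through ActiveLaser.
; While active, it spawns the laser at its own transform on BeginPlay or whenever missing on Tick, passing color, arrow and attack target.
; Tick keeps the live laser's target actor and position updated, or destroys it when inactive.
; GetHitActor forwards the laser's hit result.
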(event EventTick
  (params (DeltaSeconds :type Float%20%28single-precision%29))
  (bind _self self)
  (if (Variables|Default|GetbActiveLaser)
    (Utilities|IsValid (Variables|Default|GetChildLasers)
      (:Is%20Valid
        (Variables|/Game/Map/FX/Laser/BP_LaserFXParent.BP_LaserFXParent_C|SetbAttackActor (Variables|Default|GetChildLasers) (Variables|Default|GetbAttackActor))
        (Variables|/Game/Map/FX/Laser/BP_LaserFXParent.BP_LaserFXParent_C|SetAttackActorPos (Variables|Default|GetChildLasers) (Variables|Default|GetAttackActorPos)))
      (:Is%20Not%20Valid
        (Variables|Default|SetSpawnReference _self)
        (Variables|Default|SetID (Utilities|GetDisplayName _self))
        (bind _returnvalue (Game|SpawnActorfromClass "/Game/Map/FX/Laser/BP_LaserFX.BP_LaserFX_C" (Math|Transform|MakeTransform (.location (Transformation|GetActorTransform (Variables|Default|GetSpawnReference))) (.rotation (Transformation|GetActorTransform (Variables|Default|GetSpawnReference))) "1.000000,1.000000,1.000000") "Undefined" "MultiplyWithRoot" 0 (Variables|Default|GetArrow) (Variables|Default|GetLaserColor) (Variables|Default|GetSpawnReference) (Variables|Default|GetAttackActorPos) (Variables|Default|GetbAttackActor) 0))
        (Variables|Default|SetChildLasers _returnvalue)))
    (else
      (Utilities|IsValid (Variables|Default|GetChildLasers)
        (:Is%20Valid
          (Actor|DestroyActor (Variables|Default|GetChildLasers)))))))

(event EventBeginPlay
  (bind _self self)
  (if (Variables|Default|GetbActiveLaser)
    (Variables|Default|SetSpawnReference _self)
    (Variables|Default|SetID (Utilities|GetDisplayName _self))
    (bind _returnvalue (Game|SpawnActorfromClass "/Game/Map/FX/Laser/BP_LaserFX.BP_LaserFX_C" (Math|Transform|MakeTransform (.location (Transformation|GetActorTransform (Variables|Default|GetSpawnReference))) (.rotation (Transformation|GetActorTransform (Variables|Default|GetSpawnReference))) "1.000000,1.000000,1.000000") "Undefined" "MultiplyWithRoot" 0 (Variables|Default|GetArrow) (Variables|Default|GetLaserColor) (Variables|Default|GetSpawnReference) (Variables|Default|GetAttackActorPos) (Variables|Default|GetbAttackActor) 0))
    (Variables|Default|SetChildLasers _returnvalue)))

(fn ConstructionScript
  (|CallParentFunction))

(fn GetHitActor
  (bind _local_hit_actor (Default|GetHitActor (Variables|Default|GetChildLasers)))
  (return _local_hit_actor))