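; BP_LaserFXSpawn is a map FX actor that spawns and removes a BP_LaserFX laser according to its ActiveLaser flag.
; On BeginPlay and every Tick, it spawns the laser when active, passing itself, arrow, color and attack position, and stores it in ChildLasers.
; When ActiveLaser is off, Tick destroys the stored laser.
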(event EventTick
  (params (DeltaSeconds :type Float%20%28single-precision%29))
  (bind _self self)
  (if (Variables|Default|GetbActiveLaser)
    (Utilities|IsValid (Variables|Default|GetChildLasers)
      (:Is%20Not%20Valid
        (Variables|Default|SetSpawnReference _self)
        (Variables|Default|SetID (Utilities|GetDisplayName _self))
        (bind _returnvalue (Game|SpawnActorfromClass "/Game/Map/FX/BP_LaserFX.BP_LaserFX_C" (Math|Transform|MakeTransform "0, 0, 0" "0, 0, 0" "1.000000,1.000000,1.000000") "Undefined" "MultiplyWithRoot" 0 (Variables|Default|GetArrow) (Variables|Default|GetLaserColor) (Variables|Default|GetSpawnReference) (Variables|Default|GetAttackActorPos) 0))
        (Variables|Default|SetChildLasers _returnvalue)))
    (else
      (Utilities|IsValid (Variables|Default|GetChildLasers)
        (:Is%20Valid
          (Actor|DestroyActor (Variables|Default|GetChildLasers)))))))

(event EventBeginPlay
  (bind _self self)
  (if (Variables|Default|GetbActiveLaser)
    (Variables|Default|SetSpawnReference _self)
    (Variables|Default|SetID (Utilities|GetDisplayName _self))
    (bind _returnvalue (Game|SpawnActorfromClass "/Game/Map/FX/BP_LaserFX.BP_LaserFX_C" (Math|Transform|MakeTransform "0, 0, 0" "0, 0, 0" "1.000000,1.000000,1.000000") "Undefined" "MultiplyWithRoot" 0 (Variables|Default|GetArrow) (Variables|Default|GetLaserColor) (Variables|Default|GetSpawnReference) (Variables|Default|GetAttackActorPos) 0))
    (Variables|Default|SetChildLasers _returnvalue)))

(fn ConstructionScript
  (|CallParentFunction))