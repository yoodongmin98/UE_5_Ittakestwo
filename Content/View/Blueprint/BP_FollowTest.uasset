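; Test view actor that makes a camera follow the co-op partner's controller view between Cody and May, ticking once DoSetting is true.
; On the remote side, it finds the opposite character by the local pawn's tag, then snaps the zero-scaled camera to controller location and rotation each tick.
; On authority, it makes a one-time view-target switch between player controllers.
; DoSettingServerFunc is empty, and leftover capsule transform nodes never run.
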(event Custom|DoSettingServerFunc)

(event EventBeginPlay)

(event Collision|EventActorBeginOverlap
  (params (OtherActor :type Actor%20Object%20Reference)))

(event EventTick
  (params (DeltaSeconds :type Float%20%28single-precision%29))
  (bind _playercameracomponent (Variables|Default|GetPlayerCameraComponent))
  (bind _playercameracomponent_2 (Variables|Default|GetPlayerCameraComponent))
  (if (Variables|Default|GetDoSetting)
    (Networking|SwitchHasAuthority
      (:Authority
        (if (not (Variables|Default|GetIsClientStop))
          (Game|Player|SetViewTargetwithBlend (Game|GetPlayerController 1) (Game|GetPlayerController 2) 0.0 "VTBlend_Linear" 0.0 false)
          (Variables|Default|SetIsClientStop true)))
      (:Remote
        (Utilities|IsValid (Variables|Default|GetTarget%20Actor)
          (:Is%20Valid
            (if (Variables|Default|GetIsCody)
              (bind _asbp_cody (Utilities|Casting|CastToBP_Cody (Variables|Default|GetTarget%20Actor)))
              (Transformation|SetWorldScale3D _playercameracomponent "0, 0, 0")
              (Transformation|SetWorldRotation _playercameracomponent (Class|PlayerBase|GetCurControllerRot _asbp_cody) false false)
              (Transformation|SetWorldLocation _playercameracomponent (Class|PlayerBase|GetCurControllerLoc _asbp_cody) false true)
              (else
                (Utilities|Casting|CastToBP_May (Variables|Default|GetTarget%20Actor))
                (Transformation|SetWorldScale3D _playercameracomponent_2 "0, 0, 0")
                (Transformation|SetWorldRotation _playercameracomponent_2 (Class|PlayerBase|GetCurControllerRot) false false)
                (Transformation|SetWorldLocation _playercameracomponent_2 (Class|PlayerBase|GetCurControllerLoc) false true))))
          (:Is%20Not%20Valid
            (if (Actor|ActorHasTag (Game|Player|GetPlayerPawn 0) "May")
              (bind _returnvalue (Actor|GetActorOfClass "/Game/Characters/Cody/BP/BP_Cody.BP_Cody_C"))
              (Utilities|IsValid _returnvalue
                (:Is%20Valid
                  (Variables|Default|SetTarget%20Actor _returnvalue)
                  (Variables|Default|SetIsCody true)))
              (elif (Actor|ActorHasTag (Game|Player|GetPlayerPawn 0) "Cody")
                (bind _returnvalue_2 (Actor|GetActorOfClass "/Game/Characters/May/BP/BP_May.BP_May_C"))
                (Utilities|IsValid _returnvalue_2
                  (:Is%20Valid
                    (Variables|Default|SetTarget%20Actor _returnvalue_2)
                    (Variables|Default|SetIsCody false)))))))))))

(fn ConstructionScript)